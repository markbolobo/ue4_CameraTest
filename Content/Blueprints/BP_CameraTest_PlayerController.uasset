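; Player controller for a camera test, mapping keyboard input to character movement and cinematic camera tuning.
; Key events set held flags that TickPlayerController applies once initialized, moving the character, adjusting focal length, spring arm length and manual focus distance.
; Shift boosts camera adjustments but not movement, and manual focus unchecks the auto-focus checkbox.
; Other keys switch UI modes or toggle handheld shake through the injected UI and camera managers.
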(event `Key|One`
  (params (Key :type "Key Structure"))
  (:`Pressed`
    (`/Game/Blueprints/BP_CameraTest_UIManager.ChangeUIMode` (`self.mUIManager`) 1)))

(event `Key|Two`
  (params (Key :type "Key Structure"))
  (:`Pressed`
    (`/Game/Blueprints/BP_CameraTest_UIManager.ChangeUIMode` (`self.mUIManager`) 2)))

(event `Key|Three`
  (params (Key :type "Key Structure"))
  (:`Pressed`
    (`/Game/Blueprints/BP_CameraTest_UIManager.ChangeUIMode` (`self.mUIManager`) 3)))

(event `Key|Q`
  (params (Key :type "Key Structure"))
  (:`Pressed`
    (set `self.mIsDecreaseCameraFocalLength` true))
  (:`Released`
    (set `self.mIsDecreaseCameraFocalLength` false)))

(event `Key|W`
  (params (Key :type "Key Structure"))
  (:`Pressed`
    (set `self.mIsForward` true))
  (:`Released`
    (set `self.mIsForward` false)))

(event `Key|E`
  (params (Key :type "Key Structure"))
  (:`Pressed`
    (set `self.mIsIncreaseCameraFocalLength` true))
  (:`Released`
    (set `self.mIsIncreaseCameraFocalLength` false)))

(event `Key|A`
  (params (Key :type "Key Structure"))
  (:`Pressed`
    (set `self.mIsLeft` true))
  (:`Released`
    (set `self.mIsLeft` false)))

(event `Key|S`
  (params (Key :type "Key Structure"))
  (:`Pressed`
    (set `self.mIsBackward` true))
  (:`Released`
    (set `self.mIsBackward` false)))

(event `Key|D`
  (params (Key :type "Key Structure"))
  (:`Pressed`
    (set `self.mIsRight` true))
  (:`Released`
    (set `self.mIsRight` false)))

(event `Key|H`
  (params (Key :type "Key Structure"))
  (:`Pressed`
    (switch `ECheckBoxState` (`CheckBox.GetCheckedState` (`/Game/UI/WB_CameraTest_CameraStabilization.CheckBox_ActiveHandheld` (`/Game/Blueprints/BP_CameraTest_UIManager.mUICameraStabilization` (`self.mUIManager`))))
      (:`Unchecked`
        (`CheckBox.SetCheckedState` (`/Game/UI/WB_CameraTest_CameraStabilization.CheckBox_ActiveHandheld` (`/Game/Blueprints/BP_CameraTest_UIManager.mUICameraStabilization` (`self.mUIManager`))) "Checked")
        (set `/Game/Blueprints/CameraSystem/BP_CameraTest_CameraManager.mIsActiveHandheld` true (`self.mCameraManager`))
        (`/Game/Blueprints/CameraSystem/BP_CameraTest_CameraManager.SetHandheld` (`self.mCameraManager`)))
      (:`Checked`
        (`CheckBox.SetCheckedState` (`/Game/UI/WB_CameraTest_CameraStabilization.CheckBox_ActiveHandheld` (`/Game/Blueprints/BP_CameraTest_UIManager.mUICameraStabilization` (`self.mUIManager`))) "Unchecked")
        (set `/Game/Blueprints/CameraSystem/BP_CameraTest_CameraManager.mIsActiveHandheld` false (`self.mCameraManager`))))))

(event `Key|F`
  (params (Key :type "Key Structure"))
  (:`Pressed`
    (set `self.mIsDecreaseCameraFocusDistance` true))
  (:`Released`
    (set `self.mIsDecreaseCameraFocusDistance` false)))

(event `Key|G`
  (params (Key :type "Key Structure"))
  (:`Pressed`
    (set `self.mIsIncreaseCameraFocusDistance` true))
  (:`Released`
    (set `self.mIsIncreaseCameraFocusDistance` false)))

(event `Key|LeftShift`
  (params (Key :type "Key Structure"))
  (:`Pressed`
    (set `self.mBoost` 10.0))
  (:`Released`
    (set `self.mBoost` 1.0)))

(event `Key|Z`
  (params (Key :type "Key Structure"))
  (:`Pressed`
    (set `self.mIsDecreaseCameraSpringArm` true))
  (:`Released`
    (set `self.mIsDecreaseCameraSpringArm` false)))

(event `Key|X`
  (params (Key :type "Key Structure"))
  (:`Pressed`
    (set `self.mIsIncreaseCameraSpringArm` true))
  (:`Released`
    (set `self.mIsIncreaseCameraSpringArm` false)))

(fn `InitPlayerController`
  (params (mCharacter :type "Actor Object Reference") (mUIManager :type "/Game/Blueprints/BP_CameraTest_UIManager Object Reference") (mCameraManager :type "/Game/Blueprints/CameraSystem/BP_CameraTest_CameraManager Object Reference"))
  (set `self.mCharacter` mCharacter)
  (set `self.mUIManager` mUIManager)
  (set `self.mCameraManager` mCameraManager)
  (set `self.mSpeed` 3.0)
  (set `self.mAdjustCameraFocalLength` 0.1)
  (set `self.mAdjustCameraSpringArm` 1.0)
  (set `self.mAdjustCameraFocusDistance` 1.0)
  (set `self.mBoost` 1.0)
  (set `self.mIsInitialize` true))

(fn `TickAdjustCameraFocalLength`
  (`|ExecutionSequence`
    (:`then_0`
      (if (`self.mIsIncreaseCameraFocalLength`)
        (`/Game/Blueprints/BP_CameraTest_UIManager.AdjustCameraFocusLength` (`self.mUIManager`) (* (`self.mAdjustCameraFocalLength`) (`self.mBoost`) 1.0))))
    (:`then_1`
      (if (`self.mIsDecreaseCameraFocalLength`)
        (`/Game/Blueprints/BP_CameraTest_UIManager.AdjustCameraFocusLength` (`self.mUIManager`) (* (`self.mAdjustCameraFocalLength`) (`self.mBoost`) -1.0))))))

(fn `TickAdjustCameraFocusDistance`
  (bind _cinecamera (`/Game/Blueprints/CameraSystem/BP_CameraTest_Camera.CineCamera` (`/Game/Blueprints/CameraSystem/BP_CameraTest_CameraManager.mCamera` (`self.mCameraManager`))))
  (bind _cinecamera_2 (`/Game/Blueprints/CameraSystem/BP_CameraTest_Camera.CineCamera` (`/Game/Blueprints/CameraSystem/BP_CameraTest_CameraManager.mCamera` (`self.mCameraManager`))))
  (`|ExecutionSequence`
    (:`then_0`
      (if (`self.mIsIncreaseCameraFocusDistance`)
        (set `CineCameraComponent.FocusSettings` (make `CameraFocusSettings` "Manual" (+ (`.ManualFocusDistance` (break `CameraFocusSettings` (`CineCameraComponent.FocusSettings` _cinecamera))) (* (`self.mAdjustCameraFocusDistance`) (`self.mBoost`) 1.0)) (struct :`RelativeOffset` (0.0 0.0 0.0)) false 0.0) _cinecamera)
        (`CheckBox.SetIsChecked` (`/Game/UI/WB_CameraTest_CameraSetting.CheckBox_AutoFocus` (`/Game/Blueprints/BP_CameraTest_UIManager.mUICameraSetting` (`self.mUIManager`))) false :!label _label)))
    (:`then_1`
      (if (`self.mIsDecreaseCameraFocusDistance`)
        (set `CineCameraComponent.FocusSettings` (make `CameraFocusSettings` "Manual" (+ (`.ManualFocusDistance` (break `CameraFocusSettings` (`CineCameraComponent.FocusSettings` _cinecamera_2))) (* (`self.mAdjustCameraFocusDistance`) (`self.mBoost`) -1.0)) (struct :`RelativeOffset` (0.0 0.0 0.0)) false 0.0) _cinecamera_2)
        (goto _label)))))

(fn `TickAdjustCameraSpringArm`
  (`|ExecutionSequence`
    (:`then_0`
      (if (`self.mIsIncreaseCameraSpringArm`)
        (set `SpringArmComponent.TargetArmLength` (+ (`SpringArmComponent.TargetArmLength` (`/Game/Blueprints/CameraSystem/BP_CameraTest_CameraMode_Base.SpringArm` (`/Game/Blueprints/CameraSystem/BP_CameraTest_CameraManager.GetNowCameraMode` (`self.mCameraManager`)))) (* (`self.mAdjustCameraSpringArm`) (`self.mBoost`) 1.0)) (`/Game/Blueprints/CameraSystem/BP_CameraTest_CameraMode_Base.SpringArm` (`/Game/Blueprints/CameraSystem/BP_CameraTest_CameraManager.GetNowCameraMode` (`self.mCameraManager`))))))
    (:`then_1`
      (if (`self.mIsDecreaseCameraSpringArm`)
        (set `SpringArmComponent.TargetArmLength` (+ (`SpringArmComponent.TargetArmLength` (`/Game/Blueprints/CameraSystem/BP_CameraTest_CameraMode_Base.SpringArm` (`/Game/Blueprints/CameraSystem/BP_CameraTest_CameraManager.GetNowCameraMode` (`self.mCameraManager`)))) (* (`self.mAdjustCameraSpringArm`) (`self.mBoost`) -1.0)) (`/Game/Blueprints/CameraSystem/BP_CameraTest_CameraMode_Base.SpringArm` (`/Game/Blueprints/CameraSystem/BP_CameraTest_CameraManager.GetNowCameraMode` (`self.mCameraManager`))))))))

(fn `TickMovement`
  (bind _mcharacter (`self.mCharacter`))
  (bind _mcharacter_2 (`self.mCharacter`))
  (bind _mcharacter_3 (`self.mCharacter`))
  (bind _mcharacter_4 (`self.mCharacter`))
  ;[1 1 1] Movement
  (`|ExecutionSequence`
    (:`then_0`
      (if (`self.mIsForward`)
        (`self.K2_SetActorTransform` (`self.mCharacter`) (`KismetMathLibrary.MakeTransform` (+ (`self.K2_GetActorLocation` _mcharacter_2) (* (`self.GetActorForwardVector` _mcharacter_2) (`self.mSpeed`)))) false false)))
    (:`then_1`
      (if (`self.mIsBackward`)
        (`self.K2_SetActorTransform` (`self.mCharacter`) (`KismetMathLibrary.MakeTransform` (+ (`self.K2_GetActorLocation` _mcharacter_4) (* (* (`self.GetActorForwardVector` _mcharacter_4) -1.0) (`self.mSpeed`)))) false false)))
    (:`then_2`
      (if (`self.mIsLeft`)
        (`self.K2_SetActorTransform` (`self.mCharacter`) (`KismetMathLibrary.MakeTransform` (+ (`self.K2_GetActorLocation` _mcharacter) (* (* (`self.GetActorRightVector` _mcharacter) -1.0) (`self.mSpeed`)))) false false)))
    (:`then_3`
      (if (`self.mIsRight`)
        (`self.K2_SetActorTransform` (`self.mCharacter`) (`KismetMathLibrary.MakeTransform` (+ (`self.K2_GetActorLocation` _mcharacter_3) (* (`self.GetActorRightVector` _mcharacter_3) (`self.mSpeed`)))) false false)))))

(fn `TickPlayerController`
  (if (`self.mIsInitialize`)
    (`self.TickMovement`)
    (`self.TickAdjustCameraFocalLength`)
    (`self.TickAdjustCameraSpringArm`)
    (`self.TickAdjustCameraFocusDistance`)))

(fn `UserConstructionScript`)