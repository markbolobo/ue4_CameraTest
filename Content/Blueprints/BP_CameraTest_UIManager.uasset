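; UI manager for a camera test that creates the hint, system controller, camera setting and stabilization widgets.
; ChangeUIMode shows one of the three panels by ID, or hides it when reselected.
; TickUIManager polls widget values each call, pushing lag speed and auto focus to the camera manager and lens settings to its CineCamera, and displaying focus distance.
; AdjustCameraFocusLength nudges the focal length spin box, which the tick then applies.
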(fn `AdjustCameraFocusLength`
  (params (Amount :type "Float (double-precision)"))
  (`SpinBox.SetValue` (`/Game/UI/WB_CameraTest_CameraSetting.SpinBox_CurrentFocalLength` (`self.mUICameraSetting`)) (+ (`SpinBox.GetValue` (`/Game/UI/WB_CameraTest_CameraSetting.SpinBox_CurrentFocalLength` (`self.mUICameraSetting`))) Amount)))

(fn `ChangeUIMode`
  (params (UIID :type Integer))
  (locals (aUIID :type Integer))
  (set `local.aUIID` UIID)
  (for _array_element (`self.mAllUIs`)
    (`Widget.SetVisibility` _array_element "Hidden"))
  (if (== (`self.mUIID`) (`local.aUIID`))
    (set `self.mUIID` -1)
    (else
      (set `self.mUIID` (`local.aUIID`))
      (switch `int` (`local.aUIID`)
        (:`1`
          (`/Game/UI/WB_CameraTest_SystemController.SetUIVisibility` (`self.mUISystemController`) true))
        (:`2`
          (`/Game/UI/WB_CameraTest_CameraSetting.SetUIVisibility` (`self.mUICameraSetting`) true))
        (:`3`
          (`/Game/UI/WB_CameraTest_CameraStabilization.SetUIVisibility` (`self.mUICameraStabilization`) true))))))

(fn `InitUIManager`
  (params (mCameraManager :type "/Game/Blueprints/CameraSystem/BP_CameraTest_CameraManager Object Reference"))
  (set `self.mCameraManager` mCameraManager)
  (bind _returnvalue (`|CreateWidget` "/Game/UI/WB_CameraTest_Hint.WB_CameraTest_Hint_C"))
  (set `self.mUIHint` _returnvalue)
  (bind _returnvalue_2 (`|CreateWidget` "/Game/UI/WB_CameraTest_SystemController.WB_CameraTest_SystemController_C"))
  (bind _output_get (set `self.mUISystemController` _returnvalue_2))
  (`KismetArrayLibrary.Array_AddUnique` (`self.mAllUIs`) _output_get)
  (bind _returnvalue_3 (`|CreateWidget` "/Game/UI/WB_CameraTest_CameraSetting.WB_CameraTest_CameraSetting_C"))
  (bind _output_get_2 (set `self.mUICameraSetting` _returnvalue_3))
  (`KismetArrayLibrary.Array_AddUnique` (`self.mAllUIs`) _output_get_2)
  (bind _returnvalue_4 (`|CreateWidget` "/Game/UI/WB_CameraTest_CameraStabilization.WB_CameraTest_CameraStabilization_C"))
  (bind _output_get_3 (set `self.mUICameraStabilization` _returnvalue_4))
  (`KismetArrayLibrary.Array_AddUnique` (`self.mAllUIs`) _output_get_3)
  (`UserWidget.AddToViewport` (`self.mUIHint`) 0)
  (`UserWidget.AddToViewport` (`self.mUISystemController`) 0)
  (`UserWidget.AddToViewport` (`self.mUICameraSetting`) 0)
  (`UserWidget.AddToViewport` (`self.mUICameraStabilization`) 0)
  (`/Game/UI/WB_CameraTest_SystemController.SetUIVisibility` (`self.mUISystemController`) false)
  (`/Game/UI/WB_CameraTest_CameraSetting.SetUIVisibility` (`self.mUICameraSetting`) false)
  (`/Game/UI/WB_CameraTest_CameraStabilization.SetUIVisibility` (`self.mUICameraStabilization`) false)
  (set `self.mIsInitialize` true))

(fn `TickUICameraSetting`
  (`|ExecutionSequence`
    (:`then_0`
      (`CameraComponent.SetFieldOfView` (`/Game/Blueprints/CameraSystem/BP_CameraTest_Camera.CineCamera` (`/Game/Blueprints/CameraSystem/BP_CameraTest_CameraManager.Camera` (`self.mCameraManager`))) (`SpinBox.GetValue` (`/Game/UI/WB_CameraTest_CameraSetting.SpinBox_FieldOfView` (`self.mUICameraSetting`)))))
    (:`then_1`
      (`CineCameraComponent.SetFilmbackPresetByName` (`/Game/Blueprints/CameraSystem/BP_CameraTest_Camera.CineCamera` (`/Game/Blueprints/CameraSystem/BP_CameraTest_CameraManager.Camera` (`self.mCameraManager`))) (`ComboBoxString.GetSelectedOption` (`/Game/UI/WB_CameraTest_CameraSetting.ComboBoxString_FilmbackSetting` (`self.mUICameraSetting`)))))
    (:`then_2`
      (`CineCameraComponent.SetLensPresetByName` (`/Game/Blueprints/CameraSystem/BP_CameraTest_Camera.CineCamera` (`/Game/Blueprints/CameraSystem/BP_CameraTest_CameraManager.Camera` (`self.mCameraManager`))) (`ComboBoxString.GetSelectedOption` (`/Game/UI/WB_CameraTest_CameraSetting.ComboBoxString_LensSettings` (`self.mUICameraSetting`))))
      (set `CineCameraComponent.CurrentFocalLength` (`SpinBox.GetValue` (`/Game/UI/WB_CameraTest_CameraSetting.SpinBox_CurrentFocalLength` (`self.mUICameraSetting`))) (`/Game/Blueprints/CameraSystem/BP_CameraTest_Camera.CineCamera` (`/Game/Blueprints/CameraSystem/BP_CameraTest_CameraManager.Camera` (`self.mCameraManager`)))))
    (:`then_3`
      (set `CineCameraComponent.CurrentAperture` (`KismetStringLibrary.Conv_StringToDouble` (`ComboBoxString.GetSelectedOption` (`/Game/UI/WB_CameraTest_CameraSetting.ComboBoxString_Aperture` (`self.mUICameraSetting`)))) (`/Game/Blueprints/CameraSystem/BP_CameraTest_Camera.CineCamera` (`/Game/Blueprints/CameraSystem/BP_CameraTest_CameraManager.Camera` (`self.mCameraManager`))))
      (set `/Game/Blueprints/CameraSystem/BP_CameraTest_CameraManager.mIsAutoFocus` (`CheckBox.IsChecked` (`/Game/UI/WB_CameraTest_CameraSetting.CheckBox_AutoFocus` (`self.mUICameraSetting`))) (`self.mCameraManager`))
      (`TextBlock.SetText` (`/Game/UI/WB_CameraTest_CameraSetting.TextBlock_FocusDistance` (`self.mUICameraSetting`)) (`KismetTextLibrary.Conv_DoubleToText` (`/Game/Blueprints/CameraSystem/BP_CameraTest_CameraManager.mFocusDistance` (`self.mCameraManager`)) "HalfToEven")))))

(fn `TickUIManager`
  (if (`self.mIsInitialize`)
    (`self.TickUISystemController`)
    (`self.TickUICameraSetting`)))

(fn `TickUISystemController`
  (bind _muisystemcontroller (`self.mUISystemController`))
  (set `/Game/Blueprints/CameraSystem/BP_CameraTest_CameraManager.mCameraLagSpeed` (`KismetMathLibrary.MakeVector` (`SpinBox.GetValue` (`/Game/UI/WB_CameraTest_SystemController.SpinBox_ForwardAndBackward` _muisystemcontroller)) (`SpinBox.GetValue` (`/Game/UI/WB_CameraTest_SystemController.SpinBox_SideToSide` _muisystemcontroller)) (`SpinBox.GetValue` (`/Game/UI/WB_CameraTest_SystemController.SpinBox_UpAndDown` _muisystemcontroller))) (`self.mCameraManager`)))

(fn `UserConstructionScript`)