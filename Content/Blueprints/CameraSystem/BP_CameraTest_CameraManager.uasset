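; Camera manager for a camera test setup that spawns one camera as view target, plus TPS and aerial-view camera mode actors.
; Each tick, the current mode supplies a target location for the lagged camera, then autofocus updates.
; Handheld shake takes amplitudes from UI stabilization values, replaying through a timeline.
; Timed spring-arm adjustment exists, but its per-tick call is disconnected, so it only steps when set.
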(event `Play Handheld`
  (`Timeline|Handheld` :!via `PlayFromStart` :!label _label
    (:`Finished`
      (`self.SetHandheld`))))

(event `Stop Handheld`
  (goto _label :!via `Stop`))

(fn `ChangeCameraMode`
  (params (ID :type Integer) (CameraLagSpeed :type "Vector Structure"))
  (if (!= ID (`self.mCameraModeIndex`))
    (set `self.mCameraLagSpeed` CameraLagSpeed)
    (bind _cameralocation (`self.GetInitCameraTransform` (`self.GetNowCameraMode`)))
    (`/Game/Blueprints/CameraSystem/BP_CameraTest_Camera.InitCamera` :`self` (`self.mCamera`) :`TargetLocation` _cameralocation)))

(fn `GetInitCameraTransform`
  (params (CameraMode :type "/Game/Blueprints/CameraSystem/BP_CameraTest_CameraMode_Base Object Reference"))
  (returns (CameraLocation :type "Vector Structure"))
  (locals (aCameraLocation :type "Vector Structure"))
  (`|ExecutionSequence`
    (:`then_0`
      (bind _asbp_camera_test_camera_mode_tps (cast `/Game/Blueprints/CameraSystem/BP_CameraTest_CameraMode_TPS` (`local.CameraMode`)))
      (bind _cameralocation (`/Game/Blueprints/CameraSystem/BP_CameraTest_CameraMode_TPS.InitCameraModeTPS` _asbp_camera_test_camera_mode_tps (`self.mCharacter`)))
      (set `local.aCameraLocation` _cameralocation))
    (:`then_1`
      (bind _asbp_camera_test_camera_mode_aerial_view (cast `/Game/Blueprints/CameraSystem/BP_CameraTest_CameraMode_AerialView` (`local.CameraMode`)))
      (bind _cameralocation_2 (`/Game/Blueprints/CameraSystem/BP_CameraTest_CameraMode_AerialView.InitCameraModeAerialView` _asbp_camera_test_camera_mode_aerial_view self))
      (set `local.aCameraLocation` _cameralocation_2)))
  (return (`local.aCameraLocation`)))

(fn `GetNowCameraMode`
  (returns (NowCameraMode :type "/Game/Blueprints/CameraSystem/BP_CameraTest_CameraMode_Base Object Reference"))
  (return (`|GetArrayItem` (`self.mAllCameraMode`) (`self.mCameraModeIndex`))))

(fn `InitCameraManager`
  (params (GameManager :type "/Game/Blueprints/BP_CameraTest_GameManager Object Reference") (Character :type "Actor Object Reference") (mUIManager :type "/Game/Blueprints/BP_CameraTest_UIManager Object Reference"))
  (set `self.mGameManager` GameManager)
  (set `self.mCharacter` Character)
  (set `self.mUIManager` mUIManager)
  (`self.SpawnCamera`)
  (`self.SpawnAllCameraMode`)
  (`self.ChangeCameraMode` 1 (12.0 3.0 3.0))
  (set `self.mIsInitialize` true))

(fn `SetHandheld`
  (if (`self.mIsActiveHandheld`)
    (bind _returnvalue (`PlayerCameraManager.PlayCameraShake` :`self` (`GameplayStatics.GetPlayerCameraManager` 0) :`ShakeClass` "/Game/Blueprints/CameraSystem/BP_CameraTest_CameraShake.BP_CameraTest_CameraShake_C"))
    (`|ExecutionSequence`
      (:`then_0`
        (set `CameraShake.RotOscillation` (make `ROscillator` (make `FOscillator` (- 1.0 (`SpinBox.GetValue` (`/Game/UI/WB_CameraTest_CameraStabilization.SpinBox_Pitch` (`/Game/Blueprints/BP_CameraTest_UIManager.mUICameraStabilization` (`self.mUIManager`)))))) (make `FOscillator` (- 1.0 (`SpinBox.GetValue` (`/Game/UI/WB_CameraTest_CameraStabilization.SpinBox_Yaw` (`/Game/Blueprints/BP_CameraTest_UIManager.mUICameraStabilization` (`self.mUIManager`)))))) (make `FOscillator` (- 1.0 (`SpinBox.GetValue` (`/Game/UI/WB_CameraTest_CameraStabilization.SpinBox_Roll` (`/Game/Blueprints/BP_CameraTest_UIManager.mUICameraStabilization` (`self.mUIManager`))))))) _returnvalue))
      (:`then_1`
        (set `CameraShake.LocOscillation` (make `VOscillator` (make `FOscillator` (- 1.0 (`SpinBox.GetValue` (`/Game/UI/WB_CameraTest_CameraStabilization.SpinBox_X` (`/Game/Blueprints/BP_CameraTest_UIManager.mUICameraStabilization` (`self.mUIManager`)))))) (make `FOscillator` (- 1.0 (`SpinBox.GetValue` (`/Game/UI/WB_CameraTest_CameraStabilization.SpinBox_Y` (`/Game/Blueprints/BP_CameraTest_UIManager.mUICameraStabilization` (`self.mUIManager`)))))) (make `FOscillator` (- 1.0 (`SpinBox.GetValue` (`/Game/UI/WB_CameraTest_CameraStabilization.SpinBox_Z` (`/Game/Blueprints/BP_CameraTest_UIManager.mUICameraStabilization` (`self.mUIManager`))))))) _returnvalue))
      (:`then_2`
        (`self.Play Handheld`)))
    (else
      (`self.Stop Handheld`))))

(fn `SetSpringArm`
  (params (DelayTime :type "Float (double-precision)") (SpendTime :type "Float (double-precision)") (Speed :type "Float (double-precision)") (MinArmLength :type "Float (double-precision)") (MaxArmLength :type "Float (double-precision)") (ResetWhenFinish :type Boolean))
  (set `self.mSpringArmSpendTime` SpendTime)
  (set `self.mSpringArmSpendTick` 0.0)
  (set `self.mSpringArmAdjustSpeed` Speed)
  (set `self.mSpringArmRange` (`KismetMathLibrary.MakeVector2D` MinArmLength MaxArmLength))
  (set `self.mIsResetSpringArmWhenFinish` ResetWhenFinish)
  (set `self.mSetSpringArmDelayTime` DelayTime)
  (set `self.mSetSpringArmDelayTick` 0.0)
  (`self.TickSpringArm`))

(fn `SpawnAllCameraMode`
  (locals (TempCameraMode :type "/Game/Blueprints/CameraSystem/BP_CameraTest_CameraMode_Base Object Reference"))
  (for _array_element (`self.mCameraModeList`)
    (bind _returnvalue (`|SpawnActorFromClass` _array_element (`KismetMathLibrary.MakeTransform` (0.0 0.0 0.0)) "Undefined" "OverrideRootScale" null null))
    (set `local.TempCameraMode` _returnvalue)
    (`KismetArrayLibrary.Array_AddUnique` (`self.mAllCameraMode`) (`local.TempCameraMode`))
    (`self.GetInitCameraTransform` (`local.TempCameraMode`))
    (`/Game/Blueprints/CameraSystem/BP_CameraTest_CameraMode_Base.InitCameraBase` (`local.TempCameraMode`))))

(fn `SpawnCamera`
  (bind _returnvalue (`|SpawnActorFromClass` "/Game/Blueprints/CameraSystem/BP_CameraTest_Camera.BP_CameraTest_Camera_C" (`KismetMathLibrary.MakeTransform` (0.0 0.0 0.0)) "Undefined" "OverrideRootScale" null null))
  (bind _output_get (set `self.mCamera` _returnvalue))
  (`PlayerController.SetViewTargetWithBlend` (`GameplayStatics.GetPlayerController` 0) _output_get 0.0 "VTBlend_Linear" 0.0 false))

(fn `TickAutoFocus`
  (bind _focusdistance (`/Game/Blueprints/CameraSystem/BP_CameraTest_Camera.SetAutoFocus` (`self.mCamera`) (`self.mIsAutoFocus`)))
  (set `self.mFocusDistance` _focusdistance))

(fn `TickCameraManager`
  (params (DeltaSeconds :type "Float (double-precision)") (SpecialMotionBoost :type "Float (double-precision)"))
  (locals (aDeltaSeconds :type "Float (double-precision)") (aCameraLocation :type "Vector Structure") (aCameraRotation :type "Rotator Structure"))
  (if (`self.mIsInitialize`)
    (set `self.mDeltaSeconds` DeltaSeconds)
    (set `self.mSpecialMotionBoost` SpecialMotionBoost)
    (set `local.aDeltaSeconds` (`self.mDeltaSeconds`))
    (`|ExecutionSequence`
      (:`then_0`
        (bind _asbp_camera_test_camera_mode_tps (cast `/Game/Blueprints/CameraSystem/BP_CameraTest_CameraMode_TPS` (`self.GetNowCameraMode`)))
        (bind _cameralocation (`/Game/Blueprints/CameraSystem/BP_CameraTest_CameraMode_TPS.TickCameraModeTPS` _asbp_camera_test_camera_mode_tps))
        (set `local.aCameraLocation` _cameralocation))
      (:`then_1`
        (bind _asbp_camera_test_camera_mode_aerial_view (cast `/Game/Blueprints/CameraSystem/BP_CameraTest_CameraMode_AerialView` (`self.GetNowCameraMode`)))
        (bind _cameralocation_2 (`/Game/Blueprints/CameraSystem/BP_CameraTest_CameraMode_AerialView.TickCameraModeAerialView` _asbp_camera_test_camera_mode_aerial_view))
        (set `local.aCameraLocation` _cameralocation_2))
      (:`then_2`
        (`/Game/Blueprints/CameraSystem/BP_CameraTest_Camera.TickCamera` (`self.mCamera`) (`local.aDeltaSeconds`) (`self.mCameraLagSpeed`) (`local.aCameraLocation`) 1.0 (`local.aCameraRotation`)))
      (:`then_3`
        (`self.TickAutoFocus`)))))

(fn `TickSpringArm`
  (bind _nowcameramode (`self.GetNowCameraMode`))
  (bind (_mspringarmrange_x _mspringarmrange_y) (`KismetMathLibrary.BreakVector2D` (`self.mSpringArmRange`)))
  (bind _returnvalue (+ (`self.mSetSpringArmDelayTick`) (/ (`self.mDeltaSeconds`) (`self.mSpecialMotionBoost`))))
  (bind _returnvalue_2 (+ (`self.mSpringArmSpendTick`) (/ (`self.mDeltaSeconds`) (`self.mSpecialMotionBoost`))))
  (bind _returnvalue_3 (+ (`SpringArmComponent.TargetArmLength` (`/Game/Blueprints/CameraSystem/BP_CameraTest_CameraMode_Base.SpringArm` (`self.GetNowCameraMode`))) (`KismetMathLibrary.Lerp` 0.0 (`self.mSpringArmAdjustSpeed`) (`KismetMathLibrary.FMin` (`self.mSpringArmSpendTick`) 1.0))))
  ;[1 1 1] Delay
  (if (< _returnvalue (`self.mSetSpringArmDelayTime`))
    (set `self.mSetSpringArmDelayTick` _returnvalue)
    (else
      (if (!= (`self.mSetSpringArmDelayTime`) 0.0)
        (set `self.mSetSpringArmDelayTime` 0.0)
        (set `self.mSetSpringArmDelayTick` 0.0))
      (if (< _returnvalue_2 (`self.mSpringArmSpendTime`))
        (set `self.mSpringArmSpendTick` _returnvalue_2)
        (`/Engine/EditorBlueprintResources/StandardMacros.CompareFloat` (`self.mSpringArmAdjustSpeed`)
          (:`>`
            (set `SpringArmComponent.TargetArmLength` (`KismetMathLibrary.FMin` _returnvalue_3 _mspringarmrange_y) (`/Game/Blueprints/CameraSystem/BP_CameraTest_CameraMode_Base.SpringArm` (`self.GetNowCameraMode`))))
          (:`<`
            (set `SpringArmComponent.TargetArmLength` (`KismetMathLibrary.FMax` _returnvalue_3 _mspringarmrange_x) (`/Game/Blueprints/CameraSystem/BP_CameraTest_CameraMode_Base.SpringArm` (`self.GetNowCameraMode`)))))
        (elif (!= (`self.mSpringArmSpendTime`) 0.0)
          (set `self.mSpringArmSpendTime` 0.0)
          (set `self.mSpringArmSpendTick` 0.0)
          (set `self.mSpringArmAdjustSpeed` 0.0)
          (if (`self.mIsResetSpringArmWhenFinish`)
            (set `SpringArmComponent.TargetArmLength` (`/Game/Blueprints/CameraSystem/BP_CameraTest_CameraMode_Base.mOriginCameraLength` _nowcameramode) (`/Game/Blueprints/CameraSystem/BP_CameraTest_CameraMode_Base.SpringArm` _nowcameramode))))))))

(fn `UserConstructionScript`)