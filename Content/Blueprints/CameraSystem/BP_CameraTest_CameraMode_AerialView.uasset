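; Test camera-mode Blueprint for an aerial view in the camera system, using a StaticMesh component's world position as the output location.
; Init stores the target, snaps the actor to its location pitched straight down with a fixed yaw, and sets an initialized flag.
; The tick function returns the mesh location once initialized, without moving the actor to follow the target.
; The event graph is inactive, leaving both functions to external callers.
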(fn `InitCameraModeAerialView`
  (params (Target :type "Actor Object Reference"))
  (returns (CameraLocation :type "Vector Structure"))
  (set `self.Target` Target)
  (`self.K2_SetActorTransform` (`KismetMathLibrary.MakeTransform` (`self.K2_GetActorLocation` (`self.Target`)) (`KismetMathLibrary.MakeRotator` 0.0 -90.0 90.0)))
  (set `self.mIsInitialize` true)
  (return (`SceneComponent.K2_GetComponentLocation` (`self.StaticMesh`))))

(fn `TickCameraModeAerialView`
  (returns (CameraLocation :type "Vector Structure"))
  (if (`self.mIsInitialize`)
    (return (`SceneComponent.K2_GetComponentLocation` (`self.StaticMesh`)))))

(fn `UserConstructionScript`
  (`parent.UserConstructionScript`))