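; BP_CameraTest_CameraMode_TPS is a test third-person camera mode actor that follows a target character and supplies a world position from its StaticMesh.
; InitCameraModeTPS stores the target, snaps the actor to its location and marks it initialized.
; Once initialized, TickCameraModeTPS moves the actor to the target and returns the mesh's world location.
; Rotation handling is unwired, and its events only call the parent.
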(event `self.ReceiveBeginPlay`
  (`parent.ReceiveBeginPlay`))

(event `self.ReceiveActorBeginOverlap`
  (params (OtherActor :type "Actor Object Reference"))
  (`parent.ReceiveActorBeginOverlap` OtherActor))

(event `self.ReceiveTick`
  (params (DeltaSeconds :type "Float (single-precision)"))
  (`parent.ReceiveTick` DeltaSeconds))

(fn `InitCameraModeTPS`
  (params (TargetCharacter :type "Actor Object Reference"))
  (returns (CameraLocation :type "Vector Structure"))
  (set `self.Target` TargetCharacter)
  (`self.K2_SetActorTransform` (`KismetMathLibrary.MakeTransform` (`self.K2_GetActorLocation` (`self.Target`)) (`KismetMathLibrary.MakeRotator` 0.0)))
  (set `self.mIsInitialize` true)
  (return (`SceneComponent.K2_GetComponentLocation` (`self.StaticMesh`))))

(fn `TickCameraModeTPS`
  (returns (CameraLocation :type "Vector Structure"))
  (if (`self.mIsInitialize`)
    (`self.K2_SetActorLocation` (`self.K2_GetActorLocation` (`self.Target`)))
    (return (`SceneComponent.K2_GetComponentLocation` (`self.StaticMesh`)))))

(fn `UserConstructionScript`
  (`parent.UserConstructionScript`))