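; Test cine camera actor that follows a supplied target location and rotation with lag, driven externally through InitCamera and TickCamera.
; InitCamera snaps location using zero lag speed and enables TickCamera updates.
; Location lag interpolates each axis separately in a pitch-only rotated frame, despite comments mentioning yaw.
; Rotation lag passes RInterpTo the target as Current, so higher speeds follow less and InitCamera leaves rotation unchanged.
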(event `self.ReceiveBeginPlay`)

(event `self.ReceiveTick`
  (params (DeltaSeconds :type "Float (single-precision)")))

(fn `CameraLocationLag`
  (params (CameraLagSpeed :type "Vector Structure") (TargetLocation :type "Vector Structure"))
  (returns (Location :type "Vector Structure"))
  (bind _pitch (.pitch (`SceneComponent.K2_GetComponentRotation` (`self.CineCamera`))))
  (bind _returnvalue (`KismetMathLibrary.MakeRotator` 0.0 (* _pitch -1.0)))
  (return (`KismetMathLibrary.GreaterGreater_VectorRotator` (`KismetMathLibrary.MakeVector` (`KismetMathLibrary.FInterpTo` (.x (`KismetMathLibrary.GreaterGreater_VectorRotator` (`SceneComponent.K2_GetComponentLocation` (`self.DefaultSceneRoot`)) _returnvalue)) (.x (`KismetMathLibrary.GreaterGreater_VectorRotator` TargetLocation _returnvalue)) (`self.DeltaSeconds`) (.x CameraLagSpeed)) (`KismetMathLibrary.FInterpTo` (.y (`KismetMathLibrary.GreaterGreater_VectorRotator` (`SceneComponent.K2_GetComponentLocation` (`self.DefaultSceneRoot`)) _returnvalue)) (.y (`KismetMathLibrary.GreaterGreater_VectorRotator` TargetLocation _returnvalue)) (`self.DeltaSeconds`) (.y CameraLagSpeed)) (`KismetMathLibrary.FInterpTo` (.z (`KismetMathLibrary.GreaterGreater_VectorRotator` (`SceneComponent.K2_GetComponentLocation` (`self.DefaultSceneRoot`)) _returnvalue)) (.z (`KismetMathLibrary.GreaterGreater_VectorRotator` TargetLocation _returnvalue)) (`self.DeltaSeconds`) (.z CameraLagSpeed))) (`KismetMathLibrary.MakeRotator` 0.0 _pitch))))

(fn `CameraRotationLag`
  (params (CameraLagSpeed :type "Float (double-precision)") (TargetRotation :type "Rotator Structure"))
  (returns (Rotation :type "Rotator Structure"))
  (return (`KismetMathLibrary.RInterpTo` TargetRotation (`self.K2_GetActorRotation`) (`self.DeltaSeconds`) CameraLagSpeed)))

(fn `InitCamera`
  (params (TargetLocation :type "Vector Structure") (TargetRotation :type "Rotator Structure"))
  (set `self.mIsInitialize` true)
  (bind _location (`self.CameraLocationLag` (0.0 0.0 0.0) TargetLocation))
  (`self.K2_SetActorLocation` _location)
  (bind _rotation (`self.CameraRotationLag` 0.0 TargetRotation))
  (`self.K2_SetActorRotation` _rotation))

(fn `TickCamera`
  (params (DeltaSeconds :type "Float (double-precision)") (CameraLagSpeed :type "Vector Structure") (TargetLocation :type "Vector Structure") (CameraRotateLagSpeed :type "Float (double-precision)") (TargetRotation :type "Rotator Structure"))
  (if (`self.mIsInitialize`)
    (set `self.DeltaSeconds` DeltaSeconds)
    (bind _location (`self.CameraLocationLag` CameraLagSpeed TargetLocation))
    (`self.K2_SetActorLocation` _location)
    (bind _rotation (`self.CameraRotationLag` CameraRotateLagSpeed TargetRotation))
    (`self.K2_SetActorRotation` _rotation)))

(fn `UserConstructionScript`)