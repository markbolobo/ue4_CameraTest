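; Game manager actor for a camera test setup that bootstraps the level's core objects on BeginPlay.
; It spawns the game controller, a pawn, the camera manager and the UI manager, and fetches the first player controller as BP_CameraTest_PlayerController.
; It then injects cross-references through each one's Init function, which is skipped entirely if that controller cast fails.
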(event `self.ReceiveBeginPlay`
  (`self.InitializeGameManager`))

(fn `InitializeGameManager`
  (bind _returnvalue (`|SpawnActorFromClass` "/Game/Blueprints/BP_CameraTest_GameController.BP_CameraTest_GameController_C" (`KismetMathLibrary.MakeTransform` (0.0 0.0 0.0)) "Undefined" "OverrideRootScale" null null))
  (set `self.mGameController` _returnvalue)
  (bind _returnvalue_2 (`|SpawnActorFromClass` "/Game/Blueprints/BP_Pawn.BP_Pawn_C" (`KismetMathLibrary.MakeTransform` (0.0 0.0 100.0)) "AlwaysSpawn" "OverrideRootScale" null null))
  (set `self.mCharacter` _returnvalue_2)
  (bind _returnvalue_3 (`|SpawnActorFromClass` "/Game/Blueprints/CameraSystem/BP_CameraTest_CameraManager.BP_CameraTest_CameraManager_C" (`KismetMathLibrary.MakeTransform` (0.0 0.0 0.0)) "Undefined" "OverrideRootScale" null null))
  (set `self.mCameraManager` _returnvalue_3)
  (bind _returnvalue_4 (`|SpawnActorFromClass` "/Game/Blueprints/BP_CameraTest_UIManager.BP_CameraTest_UIManager_C" (`KismetMathLibrary.MakeTransform` (0.0 0.0 0.0)) "Undefined" "OverrideRootScale" null null))
  (set `self.mUIManager` _returnvalue_4)
  (bind _asbp_camera_test_player_controller (cast `/Game/Blueprints/BP_CameraTest_PlayerController` (`GameplayStatics.GetPlayerController` 0)))
  (set `self.mPlayerController` _asbp_camera_test_player_controller)
  (`/Game/Blueprints/BP_CameraTest_GameController.InitGameController` (`self.mGameController`) (`self.mCameraManager`) (`self.mPlayerController`) (`self.mUIManager`))
  (`/Game/Blueprints/CameraSystem/BP_CameraTest_CameraManager.InitCameraManager` (`self.mCameraManager`) self (`self.mCharacter`) (`self.mUIManager`))
  (`/Game/Blueprints/BP_CameraTest_UIManager.InitUIManager` (`self.mUIManager`) (`self.mCameraManager`))
  (`/Game/Blueprints/BP_CameraTest_PlayerController.InitPlayerController` (`self.mPlayerController`) (`self.mCharacter`) (`self.mUIManager`) (`self.mCameraManager`)))

(fn `UserConstructionScript`)