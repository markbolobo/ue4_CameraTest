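; BP_CameraTest_GameController is a central controller that drives the per-frame update of a camera test setup.
; InitGameController stores references to the camera manager, player controller and UI manager and sets an initialized flag.
; Once initialized, Tick updates those three in fixed order through their own Tick functions, passing delta time and a zero special motion boost to the camera manager.
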(event `self.ReceiveTick`
  (params (DeltaSeconds :type "Float (single-precision)"))
  (`self.TickGameController` DeltaSeconds))

(fn `InitGameController`
  (params (mCameraManager :type "/Game/Blueprints/CameraSystem/BP_CameraTest_CameraManager Object Reference") (mPlayerController :type "/Game/Blueprints/BP_CameraTest_PlayerController Object Reference") (mUIManager :type "/Game/Blueprints/BP_CameraTest_UIManager Object Reference"))
  (set `self.mIsInitialize` true)
  (set `self.mCameraManager` mCameraManager)
  (set `self.mPlayerController` mPlayerController)
  (set `self.mUIManager` mUIManager))

(fn `TickGameController`
  (params (DeltaSeconds :type "Float (double-precision)") (SpecialMotionBoost :type "Float (double-precision)"))
  (if (`self.mIsInitialize`)
    (`/Game/Blueprints/CameraSystem/BP_CameraTest_CameraManager.TickCameraManager` (`self.mCameraManager`) (`local.DeltaSeconds`) (`local.SpecialMotionBoost`))
    (`/Game/Blueprints/BP_CameraTest_PlayerController.TickPlayerController` (`self.mPlayerController`))
    (`/Game/Blueprints/BP_CameraTest_UIManager.TickUIManager` (`self.mUIManager`))))

(fn `UserConstructionScript`)